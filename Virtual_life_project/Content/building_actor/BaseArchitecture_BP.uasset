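; BaseArchitecture_BP is a building actor that turns see-through when it blocks the camera's view of the VL_metahuman player pawn.
; BeginPlay stores the mesh's first material and caches the player pawn.
; Every instance line-traces on Visibility from camera to pawn each Tick, applying Transparency_M to any BaseArchitecture_BP hit.
; An instance restores its own original material only when the trace hits no such building.
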(event EventBeginPlay
  (Variables|Default|SetOriginMateiral (Rendering|Material|GetMaterial (Variables|Default|GetSM) 0))
  (bind _asvl_metahuman (Utilities|Casting|CastToVL_metahuman (Game|Player|GetPlayerPawn 0)))
  (Variables|Default|SetPawn _asvl_metahuman))

(event EventTick
  (params (DeltaSeconds :type Float%20%28single-precision%29))
  (bind _pawn (Variables|Default|GetPawn))
  (bind _outhit (Collision|LineTraceByChannel (Transformation|GetWorldLocation (Variables|/Game/VirtualLife_Character/VL_Character.VL_Character_C|GetCamera _pawn)) (Transformation|GetActorLocation _pawn) "TraceTypeQuery1" false 0 "None" false))
  (bind _asbase_architecture_bp (Utilities|Casting|CastToBaseArchitecture_BP (.HitActor (Collision|BreakHitResult _outhit)))
    (:then
      (Rendering|Material|SetMaterial (Variables|BaseArchitecture_BP_C|GetSM _asbase_architecture_bp) 0 "/Game/building_actor/Transparency_M.Transparency_M"))
    (:CastFailed
      (Rendering|Material|SetMaterial (Variables|Default|GetSM) 0 (Variables|Default|GetOriginMateiral)))))

(fn ConstructionScript)