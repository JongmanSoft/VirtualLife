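; BP_FireSwitch is a fire prop with a point light that can be switched on and off.
; BeginPlay calls On, which raises the PointLight intensity, and the Off event sets it to zero.
; Only the light is switched: the Activate and Deactivate calls on PFire are unconnected and never run.
; Nothing in this graph calls Off.
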(event Custom|Off
  (Rendering|Components|Light|SetIntensity (Variables|Default|GetPointLight) 0.0))

(event Custom|On
  (Rendering|Components|Light|SetIntensity (Variables|Default|GetPointLight) 5e+01))

(event EventBeginPlay
  (CallFunction|On))

(event Collision|EventActorBeginOverlap
  (params (OtherActor :type Actor%20Object%20Reference)))

(event EventTick
  (params (DeltaSeconds :type Float%20%28single-precision%29)))

(fn ConstructionScript)