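; BP_StreetFireSwitch is a street fire actor that lights up at sunset and goes out at sunrise.
; NotifySunrise and NotifySunset events call Off and On, which toggle the fire particle component PFire.
; The same events switch the point light between a fixed intensity and zero, with no Tick or BeginPlay logic.
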(event Custom|Off
  (Rendering|Components|Light|SetIntensity (Variables|Default|GetPointLight) 0.0)
  (Components|Activation|Deactivate (Variables|Default|GetP_Fire)))

(event Custom|On
  (Rendering|Components|Light|SetIntensity (Variables|Default|GetPointLight) 5e+02)
  (Components|Activation|Activate (Variables|Default|GetP_Fire) false))

(event EventBeginPlay)

(event Collision|EventActorBeginOverlap
  (params (OtherActor :type Actor%20Object%20Reference)))

(event EventTick
  (params (DeltaSeconds :type Float%20%28single-precision%29)))

(event EventNotifySunrise
  (CallFunction|Off))

(event EventNotifySunset
  (CallFunction|On))

(fn ConstructionScript)