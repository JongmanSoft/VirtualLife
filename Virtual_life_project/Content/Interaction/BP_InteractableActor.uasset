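; Interactable actor that shows an interaction widget when the player enters its box and toggles an interaction state on E.
; Box overlaps use an IsPlayer message to identify the player, store the interacting actor, show or hide the lazily created widget, and enable or disable input.
; Pressing E alternates StartInteraction, which hides the widget and prints a debug string, and EndInteraction, which only clears the flag.
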(event OnComponentBeginOverlap(Box)
  (params (OverlappedComponent :type Primitive%20Component%20Object%20Reference) (OtherActor :type Actor%20Object%20Reference) (OtherComp :type Primitive%20Component%20Object%20Reference) (OtherBodyIndex :type Integer) (bFromSweep :type Boolean) (SweepResult :type Hit%20Result%20Structure%20%28by%20ref%29))
  (bind _returnvalue (Class|CharacterInterface|IsPlayer(Message) OtherActor))
  (if _returnvalue
    (Variables|Default|SetInteractingActor OtherActor)
    (Variables|Default|GetW_Interact
      (:then
        _)
      (:else
        (bind _returnvalue_2 (UserInterface|CreateWidget "/Game/Interaction/WDG_Interact.WDG_Interact_C"))
        (Variables|Default|SetW_Interact _returnvalue_2)))
    (UserInterface|Viewport|AddtoViewport (Variables|Default|GetW_Interact) 0)
    (Input|EnableInput (Game|GetPlayerController 0))))

(event OnComponentEndOverlap(Box)
  (params (OverlappedComponent :type Primitive%20Component%20Object%20Reference) (OtherActor :type Actor%20Object%20Reference) (OtherComp :type Primitive%20Component%20Object%20Reference) (OtherBodyIndex :type Integer))
  (bind _returnvalue (Class|CharacterInterface|IsPlayer(Message) OtherActor))
  (if _returnvalue
    (Utilities|HideInstruction)
    (Input|DisableInput (Game|GetPlayerController 0))))

(event Custom|StartInteraction
  (Variables|Default|SetInteracting true)
  (Utilities|HideInstruction)
  (Development|PrintString "Player Inteacting" true true "(R=0.000000,G=0.660000,B=1.000000,A=1.000000)" 1e+01))

(event Custom|EndInteraction
  (Variables|Default|SetInteracting false))

(event EventBeginPlay)

(event Collision|EventActorBeginOverlap
  (params (OtherActor :type Actor%20Object%20Reference)))

(event EventTick
  (params (DeltaSeconds :type Float%20%28single-precision%29)))

(event Input|KeyboardEvents|E
  (params (Key :type Key%20Structure :default "None"))
  (:Pressed
    (if (Variables|Default|GetInteracting)
      (CallFunction|EndInteraction)
      (else
        (CallFunction|StartInteraction)))))

(fn ConstructionScript)