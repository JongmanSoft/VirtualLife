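; Base interactable door that swings open and closed and syncs its state by door ID through Virtual_life_GameInstance.
; A box overlap shows or hides a widget for the player's VL_metahuman pawn.
; Interact alternates via FlipFlop, sending a door-state packet, playing a sound and driving a rotation timeline.
; State updates from the game instance drive a second timeline for matching IDs, independent of the FlipFlop.
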(event OnComponentBeginOverlap(Box)
  (params (OverlappedComponent :type Primitive%20Component%20Object%20Reference) (OtherActor :type Actor%20Object%20Reference) (OtherComp :type Primitive%20Component%20Object%20Reference) (OtherBodyIndex :type Integer) (bFromSweep :type Boolean) (SweepResult :type Hit%20Result%20Structure%20%28by%20ref%29))
  (if (== OtherActor (Variables|Default|GetAs%20VL%20Metahuman))
    (Rendering|SetVisibility (Variables|Default|GetWidget) true false)))

(event OnComponentEndOverlap(Box)
  (params (OverlappedComponent :type Primitive%20Component%20Object%20Reference) (OtherActor :type Actor%20Object%20Reference) (OtherComp :type Primitive%20Component%20Object%20Reference) (OtherBodyIndex :type Integer))
  (if (== OtherActor (Variables|Default|GetAs%20VL%20Metahuman))
    (Rendering|SetVisibility (Variables|Default|GetWidget) false false)))

(event Custom|update_state
  (params (door_id :type Byte%20%28by%20ref%29) (is_open :type Boolean))
  (if (== (Variables|Default|GetDoor_ID) door_id)
    (if is_open
      (Audio|PlaySound2D "/Game/EasyBuildingSystem/Audio/Sounds/Constructions/Door/SC_Door_Open.SC_Door_Open" 0.5 1.0 0.0 0 0)
      (bind _doorrotation (Timeline|Timeline Play)
        (:Update
          (Transformation|SetRelativeRotation (Variables|Default|GetSM_Door) (Math|Rotator|MakeRotator 0.0 0.0 (Math|Float|Lerp 0.0 9e+01 _doorrotation)) false false)))
      (else
        (Audio|PlaySound2D "/Game/EasyBuildingSystem/Audio/Sounds/Constructions/Door/SC_Door_Open.SC_Door_Open" 0.5 1.0 0.0 0 0)
        (Timeline|Timeline Reverse)))))

(event EventInteract
  (bind _m_inst (Variables|Default|Getm_inst))
  (Utilities|FlowControl|FlipFlop
    (:A
      (Class|VirtualLifeGameInstance|SendDoorStatePacket _m_inst (Variables|Default|GetDoor_ID) true)
      (Audio|PlaySound2D "/Game/EasyBuildingSystem/Audio/Sounds/Constructions/Door/SC_Door_Open.SC_Door_Open" 0.5 1.0 0.0 0 0)
      (bind _doorrotation (Timeline|DoorTimeLine Play)
        (:Update
          (Transformation|SetRelativeRotation (Variables|Default|GetSM_Door) (Math|Rotator|MakeRotator 0.0 0.0 (Math|Float|Lerp 0.0 9e+01 _doorrotation)) false false))))
    (:B
      (Class|VirtualLifeGameInstance|SendDoorStatePacket _m_inst (Variables|Default|GetDoor_ID) false)
      (Audio|PlaySound2D "/Game/EasyBuildingSystem/Audio/Sounds/Constructions/Door/SC_Door_Open.SC_Door_Open" 0.5 1.0 0.0 0 0)
      (Timeline|DoorTimeLine Reverse))))

(event EventBeginPlay
  (bind _asvl_metahuman (Utilities|Casting|CastToVL_metahuman (Game|Player|GetPlayerPawn 0)))
  (Variables|Default|SetAs%20VL%20Metahuman _asvl_metahuman)
  (bind _asvirtual_life_game_instance (Utilities|Casting|CastToVirtual_life_GameInstance (Game|GetGameInstance)))
  (EventDispatchers|BindEventtoUpdateDoor _asvirtual_life_game_instance (delegate Custom|update_state))
  (Variables|Default|Setm_inst _asvirtual_life_game_instance))

(fn ConstructionScript)