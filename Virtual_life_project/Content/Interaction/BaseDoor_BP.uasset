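; BaseDoor_BP is an interactable door that swings open and closed and shows a widget while the player is near.
; It caches the VL_metahuman player pawn on BeginPlay, and Box overlap events toggle the widget's visibility for that pawn only.
; Interact plays a door sound, then a FlipFlop alternately plays and reverses a timeline that lerps the door mesh's relative yaw through a quarter turn.
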(event OnComponentBeginOverlap(Box)
  (params (OverlappedComponent :type Primitive%20Component%20Object%20Reference) (OtherActor :type Actor%20Object%20Reference) (OtherComp :type Primitive%20Component%20Object%20Reference) (OtherBodyIndex :type Integer) (bFromSweep :type Boolean) (SweepResult :type Hit%20Result%20Structure%20%28by%20ref%29))
  (if (== OtherActor (Variables|Default|GetAs%20VL%20Metahuman))
    (Rendering|SetVisibility (Variables|Default|GetWidget) true false)))

(event OnComponentEndOverlap(Box)
  (params (OverlappedComponent :type Primitive%20Component%20Object%20Reference) (OtherActor :type Actor%20Object%20Reference) (OtherComp :type Primitive%20Component%20Object%20Reference) (OtherBodyIndex :type Integer))
  (if (== OtherActor (Variables|Default|GetAs%20VL%20Metahuman))
    (Rendering|SetVisibility (Variables|Default|GetWidget) false false)))

(event EventBeginPlay
  (bind _asvl_metahuman (Utilities|Casting|CastToVL_metahuman (Game|Player|GetPlayerPawn 0)))
  (Variables|Default|SetAs%20VL%20Metahuman _asvl_metahuman))

(event EventInteract
  (Audio|PlaySound2D "/Game/sound/effect_sound/door.door" 1.0 1.0 0.0 0 0)
  (Utilities|FlowControl|FlipFlop
    (:A
      (bind _doorrotation (Timeline|DoorTimeLine Play)
        (:Update
          (Transformation|SetRelativeRotation (Variables|Default|GetSM_Door) (Math|Rotator|MakeRotator 0.0 0.0 (Math|Float|Lerp 0.0 9e+01 _doorrotation)) false false))))
    (:B
      (Timeline|DoorTimeLine Reverse))))

(fn ConstructionScript)