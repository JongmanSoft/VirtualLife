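; Placement preview actor for the building system that shows a glowing ghost of the chosen building mesh under the mouse cursor.
; Each tick, a 2000-unit visibility trace from the deprojected cursor finds the hit point, which is snapped to the grid to position the mesh with the current yaw.
; PlaceBuild spawns a PlaceBuild_BP at that location and rotation, passing it the building mesh.
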(event EventBeginPlay
  (bind _mesh (Variables|Default|GetMesh))
  (Components|StaticMesh|SetStaticMesh _mesh (Variables|Default|GetBuildingMesh))
  (Rendering|Material|SetOverlayMaterial _mesh "/Game/BuildingSystem/Glow_M.Glow_M" :!class /Script/Engine.MeshComponent))

(event EventTick
  (params (DeltaSeconds :type Float%20%28single-precision%29))
  (bind _returnvalue (CallFunction|MousePosition))
  (bind _output_get (Variables|Default|SetLocationOfMesh _returnvalue))
  (Transformation|SetWorldTransform (Variables|Default|GetMesh) (Math|Transform|MakeTransform (Class|KismetMathLibrary|VectorSnappedtoGrid _output_get (Variables|Default|GetGridSize)) (Math|Rotator|MakeRotator 0.0 0.0 (Variables|Default|GetRotate)) "1.000000,1.000000,1.000000") false false))

(fn ConstructionScript)

(fn MousePosition
  (bind _returnvalue (Game|GetPlayerController 0))
  (bind (_worldlocation _worlddirection) (Game|Player|ConvertMouseLocationToWorldSpace _returnvalue))
  (bind (_outhit _returnvalue_2) (Collision|LineTraceByChannel _worldlocation (+ _worldlocation (* _worlddirection 2e+03)) "TraceTypeQuery1" false 0 "None"))
  (if _returnvalue_2
    (return (Class|KismetMathLibrary|VectorSnappedtoGrid (.Location (Collision|BreakHitResult _outhit)) (Variables|Default|GetGridSize)))))

(fn PlaceBuild
  (Game|SpawnActorfromClass "/Game/BuildingSystem/Actors/PlaceBuild_BP.PlaceBuild_BP_C" (Math|Transform|MakeTransform (Variables|Default|GetLocationOfMesh) (Math|Rotator|MakeRotator 0.0 0.0 (Variables|Default|GetRotate)) "1.000000,1.000000,1.000000") "Undefined" "MultiplyWithRoot" 0 (Variables|Default|GetBuildingMesh) 0))